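; BPTile00 is a board tile Blueprint that reacts to the mouse cursor in a dice-and-pawns game.
; On cursor over, it reads the BPGameState phase and moves its Highlight component to just above the TileMesh.
; The phase switch covers player count selection, dice throwing and pawn movement, but its branches are empty.
; The click event and construction script are stubs.
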(event OnClicked(TileMesh)
  (params (TouchedComponent :type Primitive%20Component%20Object%20Reference)))

(event OnBeginCursorOver(TileMesh)
  (params (TouchedComponent :type Primitive%20Component%20Object%20Reference))
  (bind _tilemesh (Variables|Default|GetTileMesh))
  (bind _relativelocation (Variables|/Script/Engine.SceneComponent|GetRelativeLocation _tilemesh))
  (bind (_x _y _z) (Math|Vector|BreakVector _relativelocation))
  (bind _asbpgame_state (Utilities|Casting|CastToBPGameState (Game|GetGameState)))
  (switch Utilities|FlowControl|Switch|SwitchonEGameState (Variables|/Game/Blueprints/BPGameState.BPGameState_C|GetState _asbpgame_state)
    (:NewEnumerator0
      _)
    (:NewEnumerator1
      _)
    (:NewEnumerator2
      _))
  (Transformation|SetActorRelativeLocation (Variables|Default|GetHighlight) (Math|Vector|MakeVector _x _y (+ _z 5.0))))

(fn ConstructionScript)