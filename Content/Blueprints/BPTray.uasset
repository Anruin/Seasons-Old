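; Dice tray that handles the player's roll and plays impact sounds.
; Releasing RollDice fires the DiceShaker impulse, flags the roll on BPGameState, then copies both TargetDice results into its DiceValue after a fixed delay, without checking that the dice have settled.
; Hit events choose one of four sounds by impulse magnitude, with randomized pitch, and ignore very weak contacts.
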(event EventHit
  (params (MyComp :type Primitive%20Component%20Object%20Reference) (Other :type Actor%20Object%20Reference) (OtherComp :type Primitive%20Component%20Object%20Reference) (bSelfMoved :type Boolean) (HitLocation :type Vector :default "0, 0, 0") (HitNormal :type Vector :default "0, 0, 0") (NormalImpulse :type Vector :default "0, 0, 0") (Hit :type Hit%20Result%20Structure%20%28by%20ref%29))
  (bind _returnvalue (Math|Vector|VectorLength NormalImpulse))
  (bind _returnvalue_2 (Math|Random|RandomFloatinRange 0.75 1.25))
  ;[1 1 1] Dice hit sounds
  (if (and (> _returnvalue 5e+01) (<= _returnvalue 1.5e+02))
    (Audio|PlaySoundatLocation (Variables|Default|GetSoundHitSIlent) HitLocation (Variables|Default|GetVolumeHitSilent) _returnvalue_2)
    (elif (and (> _returnvalue 1.5e+02) (<= _returnvalue 5e+02))
      (Audio|PlaySoundatLocation (Variables|Default|GetSoundHitQuiet) HitLocation (Variables|Default|GetVolumeHitQuiet) _returnvalue_2)
      (elif (and (> _returnvalue 5e+02) (<= _returnvalue 2.5e+03))
        (Audio|PlaySoundatLocation (Variables|Default|GetSoundHitNormal) HitLocation (Variables|Default|GetVolumeHitNormal) _returnvalue_2)
        (elif (> _returnvalue 2.5e+03)
          (Audio|PlaySoundatLocation (Variables|Default|GetSoundHitLoud) HitLocation (Variables|Default|GetVolumeHitLoud) _returnvalue_2))))))

(event EventBeginPlay
  (Input|EnableInput (Game|GetPlayerController 0)))

(event Input|ActionEvents|InputActionRollDice
  (bind _targetdice (Variables|Default|GetTargetDice))
  ;[1 1 1] Main logic
  (:Released
    (Class|RadialForceComponent|FireImpulse (Variables|Default|GetDiceShaker))
    (bind _asbpgame_state (Utilities|Casting|CastToBPGameState (Game|GetGameState))
      (:then
        (Variables|/Game/Blueprints/BPGameState.BPGameState_C|SetDiceRolled _asbpgame_state true)
        (Utilities|FlowControl|Delay 2.0)
        (bind _asbpdice (Utilities|Casting|CastToBPDice (Utilities|Array|Get(acopy) _targetdice))
          (:then
            (bind _asbpdice_2 (Utilities|Casting|CastToBPDice (Utilities|Array|Get(acopy) _targetdice 1))
              (:then
                (Variables|/Game/Blueprints/BPGameState.BPGameState_C|SetDiceValue _asbpgame_state (Utilities|Array|MakeArray (Variables|/Game/Blueprints/BPDice.BPDice_C|GetDiceResultData _asbpdice) (Variables|/Game/Blueprints/BPDice.BPDice_C|GetDiceResultData _asbpdice_2))))
              (:CastFailed
                (Development|PrintString "Cast failed" :!label _label))))
          (:CastFailed
            (goto _label))))
      (:CastFailed
        (goto _label)))))

(fn ConstructionScript)